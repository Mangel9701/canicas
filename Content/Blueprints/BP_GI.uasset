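; BP_GI, by its name a Game Instance Blueprint, shows and hides the game's pause screen.
; PauseGame creates the PAUSE widget, adds it to the viewport and pauses the game, while ReturnGame unpauses and removes the widget.
; Both events update the PauseMenu flag and share a final step that sets mouse cursor visibility from it.
; A branch that checks PauseMenu before pausing is left unconnected and never runs.
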(event `ReturnGame`
  ;[1 1 1] Show Pause game screen
  (`GameplayStatics.SetGamePaused` false) ; Toggle Game Status
  (`Widget.RemoveFromParent` (stale `PauseGame` _returnvalue))
  (set `self.bPauseMenu` false)
  (set `PlayerController.bShowMouseCursor` (`self.bPauseMenu`) (`GameplayStatics.GetPlayerController` 0) :!label _label))

(event `PauseGame`
  ;[1 1 1] Show Pause game screen
  (bind _returnvalue (`|CreateWidget` "/Game/FirstPersonBP/Maps/PAUSE.PAUSE_C" (`GameplayStatics.GetPlayerController` 0)))
  (`UserWidget.AddToViewport` _returnvalue 0)
  (`GameplayStatics.SetGamePaused` true) ; Toggle Game Status
  (set `self.bPauseMenu` true)
  (goto _label))