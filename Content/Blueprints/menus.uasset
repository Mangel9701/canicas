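; Menus Blueprint that shows and hides the game's pause screen.
; PauseGame creates a PAUSE widget for the first player controller, adds it to the viewport and pauses the game.
; ReturnGame unpauses and removes that stored widget.
; Disconnected nodes that would set a PauseMenu flag and mouse cursor visibility never run, and the construction script is empty.
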(event `ReturnGame`
  ;[1 1 1] Show Pause game screen
  (`GameplayStatics.SetGamePaused` false) ; Toggle Game Status
  (`Widget.RemoveFromParent` (stale `PauseGame` _returnvalue)))

(event `PauseGame`
  ;[1 1 1] Show Pause game screen
  (bind _returnvalue (`|CreateWidget` "/Game/FirstPersonBP/Maps/PAUSE.PAUSE_C" (`GameplayStatics.GetPlayerController` 0)))
  (`UserWidget.AddToViewport` _returnvalue 0)
  (`GameplayStatics.SetGamePaused` true) ; Toggle Game Status
)

(fn `UserConstructionScript`)